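; BP_ShotgunsMaster is a master Blueprint for modular shotguns, assembled from boolean options with no active event logic.
; Its construction script first applies shared color, camo, metallic and roughness values through dynamic material instances on material slot 0.
; It then destroys unselected pre-placed meshes across barrel, fore-end, stock, rail and sight groups.
; Some options are nested, so supports, grips and fast-reload shells depend on their parent part.
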(event EventBeginPlay)

(event Collision|EventActorBeginOverlap
  (params (OtherActor :type Actor%20Object%20Reference)))

(event EventTick
  (params (DeltaSeconds :type Float%20%28single-precision%29)))

(fn ConstructionScript
  (CallFunction|Color)
  (Utilities|FlowControl|Sequence
    (:then_0
      ;[1 1 1] Barrel
      (Utilities|FlowControl|Sequence
        (:then_0
          (if (Variables|Barrel|GetBarrel%20Comum)
            (Components|DestroyComponent (Variables|Default|GetSM_B3_BarrelLong))
            ;[1 1 1] Supports
            (Components|DestroyComponent (Variables|Default|GetSM_H1_2_SuportBarrelPart_Rail))
            (else
              (Components|DestroyComponent (Variables|Default|GetSM_B2_BarrelComum)))))
        (:then_1
          (if (Variables|Barrel|GetBarrel%20Classic)
            (Components|DestroyComponent (Variables|Default|GetSM_B2_BarrelComum))
            (Utilities|FlowControl|Sequence :!label _label
              (:then_0
                (if (Variables|Supports|GetFront%20Support%20Tactical)
                  (Components|DestroyComponent (Variables|Default|GetSM_H2_SuportBarrelPart))
                  (else
                    (Components|DestroyComponent (Variables|Default|GetSM_H1_1_SuportBarrelPart_Tactical))))
                (if (not (Variables|Supports|GetFront%20Support%20%28Rail%29))
                  (Components|DestroyComponent (Variables|Default|GetSM_H1_2_SuportBarrelPart_Rail))))
              (:then_1
                (if (Variables|Supports|GetFront%20Support%20Comum)
                  (Components|DestroyComponent (Variables|Default|GetSM_H1_1_SuportBarrelPart_Tactical))
                  (else
                    (Components|DestroyComponent (Variables|Default|GetSM_H2_SuportBarrelPart))))
                (if (not (Variables|Supports|GetCloak))
                  (Components|DestroyComponent (Variables|Default|GetSM_I1_Cloak)))))
            (else
              (Components|DestroyComponent (Variables|Default|GetSM_B1_BarrelClassic)))))
        (:then_2
          (if (Variables|Barrel|GetBarrel%20Tactical)
            (Components|DestroyComponent (Variables|Default|GetSM_B1_BarrelClassic))
            (goto _label)
            (else
              (Components|DestroyComponent (Variables|Default|GetSM_B4_BarrelTactical)))))
        (:then_3
          (if (Variables|Barrel|GetBarrel%20Long)
            (Components|DestroyComponent (Variables|Default|GetSM_B1_BarrelClassic))
            (goto _label)
            (else
              (Components|DestroyComponent (Variables|Default|GetSM_B3_BarrelLong)))))))
    (:then_1
      ;[1 1 1] Fore-end
      (Utilities|FlowControl|Sequence
        (:then_0
          (if (Variables|Fore-End|GetFore-end%20Classic)
            (Components|DestroyComponent (Variables|Default|GetSM_C3_PumpPolice))
            (else
              (Components|DestroyComponent (Variables|Default|GetSM_C2_PumpClassic)))))
        (:then_1
          (if (Variables|Fore-End|GetFore-end%20Police)
            (Components|DestroyComponent (Variables|Default|GetSM_C2_PumpClassic))
            (else
              (Components|DestroyComponent (Variables|Default|GetSM_C3_PumpPolice)))))
        (:then_2
          (if (Variables|Fore-End|GetFore-end%20Camo)
            (Components|DestroyComponent (Variables|Default|GetSM_C2_PumpClassic))
            (else
              (Components|DestroyComponent (Variables|Default|GetSM_C1_PumpCamo)))))
        (:then_3
          (if (Variables|Fore-End|GetFore-end%20Tactical)
            (Components|DestroyComponent (Variables|Default|GetSM_C2_PumpClassic))
            (else
              (Components|DestroyComponent (Variables|Default|GetSM_C4_PumpTactical)))))))
    (:then_2
      ;[1 1 1] Stock
      (Utilities|FlowControl|Sequence
        (:then_0
          (if (Variables|Stock/Grip|GetStock%20Classic)
            (Components|DestroyComponent (Variables|Default|GetSM_E2_StockPolice))
            (Components|DestroyComponent (Variables|Default|GetSM_F2_PistolGripTactical) :!label _label_2)
            (else
              (Components|DestroyComponent (Variables|Default|GetSM_E5_StockClassic)))))
        (:then_1
          (if (Variables|Stock/Grip|GetStock%20Police)
            (Components|DestroyComponent (Variables|Default|GetSM_E5_StockClassic))
            ;[1 1 1] Grip
            (if (Variables|Stock/Grip|GetGrip%20Police/Tactical) :!label _label_3
              (Components|DestroyComponent (Variables|Default|GetSM_F1_PistolGripPolice))
              (else
                (Components|DestroyComponent (Variables|Default|GetSM_F2_PistolGripTactical))))
            (else
              (Components|DestroyComponent (Variables|Default|GetSM_E2_StockPolice)))))
        (:then_2
          (if (Variables|Stock/Grip|GetStock%20Camo)
            (Components|DestroyComponent (Variables|Default|GetSM_E5_StockClassic))
            (goto _label_2)
            (else
              (Components|DestroyComponent (Variables|Default|GetSM_E1_StockCamo)))))
        (:then_3
          (if (Variables|Stock/Grip|GetStock%20Tactical)
            (Components|DestroyComponent (Variables|Default|GetSM_E5_StockClassic))
            (goto _label_2)
            (else
              (Components|DestroyComponent (Variables|Default|GetSM_E3_StockTactical)))))
        (:then_4
          (if (Variables|Stock/Grip|GetStock%20Tactical%20Camo)
            (Components|DestroyComponent (Variables|Default|GetSM_E5_StockClassic))
            (goto _label_3)
            (else
              (Components|DestroyComponent (Variables|Default|GetSM_E4_StockTacticalCamo)))))))
    (:then_3
      ;[1 1 1] Rail Barrel
      (Utilities|FlowControl|Sequence
        (:then_0
          (if (Variables|RailBarrel|GetRail%20Barrel%20Tactical)
            (Components|DestroyComponent (Variables|Default|GetSM_D1_RailBarrelUniquePart))
            (if (Variables|RailBarrel|GetFast%20Reload)
              (if (not (Variables|RailBarrel|GetAmmo))
                (Components|DestroyComponent (Variables|Default|GetSM_D3_2_1_12BulletFR_01) :!label _label_4))
              (else
                (Components|DestroyComponent (Variables|Default|GetSM_D3_2_FastReloadPart) :!label _label_5)
                (goto _label_4)))
            (else
              (Components|DestroyComponent (Variables|Default|GetSM_D3_1_RailBarrelTactical))
              (goto _label_5))))
        (:then_1
          (if (Variables|RailBarrel|GetRail%20Barrel%20Comum)
            (Components|DestroyComponent (Variables|Default|GetSM_D3_1_RailBarrelTactical))
            (else
              (Components|DestroyComponent (Variables|Default|GetSM_D1_RailBarrelUniquePart)))))
        (:then_2
          (if (Variables|RailBarrel|GetRail%20Barrel%20Float)
            (Components|DestroyComponent (Variables|Default|GetSM_D3_1_RailBarrelTactical))
            (else
              (Components|DestroyComponent (Variables|Default|GetSM_D2_1_RailBarrelPart_01)))))
        (:then_3
          (if (Variables|RailBarrel|GetRail%20Barrel%20SupportSight)
            (Components|DestroyComponent (Variables|Default|GetSM_D3_1_RailBarrelTactical))
            (else
              (Components|DestroyComponent (Variables|Default|GetSM_D2_2_RailBarrelPart_02)))))
        (:then_4
          (if (not (Variables|RailBarrel|GetRail%20Barrel%20Body))
            (Components|DestroyComponent (Variables|Default|GetSM_D4_RailBody))))))
    (:then_4
      ;[1 1 1] Sights
      (Utilities|FlowControl|Sequence
        (:then_0
          (if (Variables|MetalSight|GetMetal%20Sight%20%28Only%20Barrel%29)
            (Components|DestroyComponent (Variables|Default|GetSM_G2_SightMetalBarrel))
            (else
              (Components|DestroyComponent (Variables|Default|GetSM_G1_1_SightUniquePart_03)))))
        (:then_1
          (if (Variables|MetalSight|GetMetal%20Sight)
            (Components|DestroyComponent (Variables|Default|GetSM_G1_1_SightUniquePart_03))
            (else
              (Components|DestroyComponent (Variables|Default|GetSM_G2_SightMetalBarrel)))))))))

(fn SetColorFunction
  (params (InputPin :type Material%20Instance%20Dynamic%20Object%20Reference))
  (Rendering|Material|SetVectorParameterValue InputPin "Color" (Variables|Default|GetMain%20Metal) :!class /Script/Engine.MaterialInstanceDynamic)
  (Rendering|Material|SetVectorParameterValue InputPin "ColorCamo" (Variables|Default|GetMain%20Camo) :!class /Script/Engine.MaterialInstanceDynamic)
  (Rendering|Material|SetScalarParameterValue InputPin "MET" (Variables|Default|GetMetallic) :!class /Script/Engine.MaterialInstanceDynamic)
  (Rendering|Material|SetScalarParameterValue InputPin "ROUGH" (Variables|Default|GetRoughness) :!class /Script/Engine.MaterialInstanceDynamic))

(fn SetSMsbyColor
  (params (Array :type Array%20of%20Primitive%20Component%20Object%20References) (ElementIndex :type Integer))
  (for _array_element Array
    (bind _returnvalue (Rendering|Material|CreateDynamicMaterialInstance _array_element ElementIndex 0 "None" :!class /Script/Engine.PrimitiveComponent))
    (CallFunction|SetColorFunction _returnvalue))
  (return))

(fn Color
  (CallFunction|SetSMsbyColor (|SMMATIndex0)))